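; Coin pickup actor that can be hidden when picked and brought back on restore, with a save step that locks in collected coins.
; Picked sets Grabbed and hides the actor, while Save allows respawn only for coins not yet grabbed.
; Restore unhides the coin and clears Grabbed only if CanRespawn is set.
; The event graph and construction script are empty, so these functions contain all the logic.
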(fn `Picked`
  (bind _output_get (set `self.Grabbed` true))
  (`self.SetActorHiddenInGame` _output_get))

(fn `Restore`
  (if (`self.CanRespawn`)
    (`self.SetActorHiddenInGame` false)
    (set `self.Grabbed` false)))

(fn `Save`
  (if (`self.Grabbed`)
    (set `self.CanRespawn` false)
    (else
      (set `self.CanRespawn` true))))

(fn `UserConstructionScript`)
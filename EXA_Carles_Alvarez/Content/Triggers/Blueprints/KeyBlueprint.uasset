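; Key pickup actor that the ThirdPersonCharacter collects by overlapping its Box.
; Overlap disables collision, hides the actor and sets Picked, which makes Tick print "Key" every frame.
; Separate, locally uncalled functions manage checkpoint-style state: PickedKey sets Grabbed and hides, Save allows respawn only for ungrabbed keys.
; RestoreKey unhides respawnable keys and clears Grabbed, leaving Picked and collision unchanged.
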(event `self.ReceiveTick`
  (params (DeltaSeconds :type "Float (single-precision)"))
  ;[0 1 0.4066] Si se recoge se printea
  (if (`self.Picked`)
    (`KismetSystemLibrary.PrintString` "Key" true true (struct :`G` 0.66 :`B` 1.0 :`A` 1.0) 0.0)))

(event `self.Box.OnComponentBeginOverlap`
  (params (OverlappedComponent :type "PrimitiveComponent Object Reference") (OtherActor :type "Actor Object Reference") (OtherComp :type "PrimitiveComponent Object Reference") (OtherBodyIndex :type Integer) (bFromSweep :type Boolean) (SweepResult :type "HitResult Structure (by ref)"))
  ;[1 0 0] Si colisiona se activa
  (cast `/Game/Triggers/Blueprints/ThirdPersonCharacter` OtherActor)
  (`self.SetActorEnableCollision` false)
  (`self.SetActorHiddenInGame` true)
  (set `self.Picked` true))

(fn `PickedKey`
  (bind _output_get (set `self.Grabbed` true))
  (`self.SetActorHiddenInGame` _output_get))

(fn `Restore Key`
  (if (`self.CanRespawn`)
    (`self.SetActorHiddenInGame` false)
    (set `self.Grabbed` false)))

(fn `Save`
  (if (`self.Grabbed`)
    (set `self.CanRespawn` false)
    (else
      (set `self.CanRespawn` true))))

(fn `UserConstructionScript`)
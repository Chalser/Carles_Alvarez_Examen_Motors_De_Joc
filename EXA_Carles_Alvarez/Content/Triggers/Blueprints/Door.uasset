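; Door actor that slides open once the third-person player character holds exactly three coins.
; BeginPlay caches the door's starting location and a reference to the player character.
; Tick polls the coin count and plays the OpenSesamee timeline, which lerps the static mesh from the start location by the End offset, without sweep.
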(event `self.ReceiveBeginPlay`
  (set `self.Start` (`self.K2_GetActorLocation`))
  (bind _asthird_person_character (cast `/Game/Triggers/Blueprints/ThirdPersonCharacter` (`GameplayStatics.GetPlayerPawn` 0)))
  (set `self.Player` _asthird_person_character))

(event `self.ReceiveTick`
  (params (DeltaSeconds :type "Float (single-precision)"))
  (if (== (`/Game/Triggers/Blueprints/ThirdPersonCharacter.Coins` (`self.Player`)) 3.0)
    (bind (_direction _newtrack_0) (`Timeline|Open Sesamee`)
      (:`Update`
        (`SceneComponent.K2_SetWorldLocation` (`self.StaticMesh`) (`KismetMathLibrary.VLerp` (`self.Start`) (+ (`self.Start`) (`self.End`)) _newtrack_0) false false)))))

(fn `UserConstructionScript`)